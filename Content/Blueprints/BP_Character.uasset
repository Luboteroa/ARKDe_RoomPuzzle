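; BP_Character is a character Blueprint with switchable first- or third-person view, jump signalling and melee overlap detection.
; The construction script uses UseFirstPersonView to set which camera components auto-activate: FPS, or TPS with spring arm.
; BeginPlay caches the mesh's ABP_Character anim instance, whose CanJump flag the Jump event pulses briefly.
; The melee detector only prints the name of overlapping actors.
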(event OnComponentBeginOverlap(MeleeDetectorComponent)
  (params (OverlappedComponent :type Primitive%20Component%20Object%20Reference) (OtherActor :type Actor%20Object%20Reference) (OtherComp :type Primitive%20Component%20Object%20Reference) (OtherBodyIndex :type Integer) (bFromSweep :type Boolean) (SweepResult :type Hit%20Result%20Structure%20%28by%20ref%29))
  (Development|PrintString (Utilities|GetDisplayName OtherActor)))

(event EventBeginPlay
  (bind _asabp_character (Utilities|Casting|CastToABP_Character (Components|SkeletalMesh|GetAnimInstance (Variables|Character|GetMesh))))
  (Variables|Default|SetAs%20ABP%20Character _asabp_character))

(event EventJump
  (Variables|/Game/Animations/Character/ABP_Character.ABP_Character_C|SetCan%20Jump (Variables|Default|GetAs%20ABP%20Character) true)
  (Utilities|FlowControl|Delay 0.2)
  (Variables|/Game/Animations/Character/ABP_Character.ABP_Character_C|SetCan%20Jump (Variables|Default|GetAs%20ABP%20Character) false))

(fn ConstructionScript
  (Components|Activation|SetAutoActivate (Variables|Default|GetFPSCameraComponent) (Variables|Default|GetUse%20First%20Person%20View))
  (Components|Activation|SetAutoActivate (Variables|Default|GetTPSCameraComponent) (not (Variables|Default|GetUse%20First%20Person%20View))))