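; BP_NewLandMine is a landmine that stays invisible until its warning zone is entered.
; It sets the mesh material's Opacity parameter to zero at BeginPlay and on zone exit, and to partly visible on zone entry.
; TriggerExplosion swaps the mesh to an opaque material, with no damage or effects in this graph.
; Each warning and explosion event prints a colored on-screen message.
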(event EventBeginPlay
  (Rendering|Material|SetScalarParameterValueonMaterials (Variables|Default|GetMeshComponent) "Opacity" 0.0))

(event EventOnWarningZoneEnter
  (Rendering|Material|SetScalarParameterValueonMaterials (Variables|Default|GetMeshComponent) "Opacity" 0.35)
  (Development|PrintString "Entering on landmine zone D:" true true "(R=1.000000,G=0.672742,B=0.000000,A=1.000000)"))

(event EventOnWarningZoneExit
  (Rendering|Material|SetScalarParameterValueonMaterials (Variables|Default|GetMeshComponent) "Opacity" 0.0)
  (Development|PrintString "Exiting landmine zone :D" true true "(R=0.821500,G=0.000000,B=1.000000,A=1.000000)"))

(event EventTriggerExplosion
  (Rendering|Material|SetMaterial (Variables|Default|GetMeshComponent) 0 "/Game/Landmine/model/textures/Landmine_Opaque.Landmine_Opaque")
  (Development|PrintString "BOOM!" true true "(R=0.000000,G=1.000000,B=0.057209,A=1.000000)"))

(fn ConstructionScript)