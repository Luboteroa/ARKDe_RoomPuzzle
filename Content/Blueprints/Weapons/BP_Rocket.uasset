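; BP_Rocket is a rocket weapon Blueprint that holds an unfinished targeting stub.
; Its Targeting event only prints the display name of the ComponentTargeted variable to the screen.
; An unconnected camera-forward visibility line trace with debug drawing reads the hit component but never runs, and the construction script is empty.
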(event EventTargeting
  (Development|PrintString (Utilities|GetDisplayName (Variables|Default|GetComponentTargeted))))

(fn ConstructionScript)